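; Gateporter_2 is a rotating gateway that ends the level and loads another map.
; When a FlyingPawn overlaps the Box while not carrying a star and ObjComplete is true, it sets Victory.
; After a delay, it opens the level named in MapToGOTO.
; Tick spins the Gateway component by a fixed local rotation each frame, without delta-time scaling.
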(event OnComponentBeginOverlap(Box)
  (params (OverlappedComponent :type Primitive%20Component%20Object%20Reference) (OtherActor :type Actor%20Object%20Reference) (OtherComp :type Primitive%20Component%20Object%20Reference) (OtherBodyIndex :type Integer) (bFromSweep :type Boolean) (SweepResult :type Hit%20Result%20Structure%20%28by%20ref%29))
  ;[1 1 1] Functionality
  (bind _asflying_pawn (Utilities|Casting|CastToFlyingPawn OtherActor))
  (if (not (Variables|/Game/FlyingBP/Blueprints/FlyingPawn.FlyingPawn_C|GetbHasStar? _asflying_pawn))
    (if (Variables|Default|GetObjComplete)
      (Variables|Default|Setvictory true)
      (Utilities|FlowControl|Delay 1e+01)
      (Game|OpenLevel(byName) (Variables|Default|GetMapToGOTO)))))

(event EventTick
  (params (DeltaSeconds :type Float%20%28single-precision%29))
  ;[1 1 1] Rotation
  (Transformation|AddLocalRotation (Variables|Default|GetGateway) "0,0.025000, 0" false false))

(fn ConstructionScript)