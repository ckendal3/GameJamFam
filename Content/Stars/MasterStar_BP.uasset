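; Base star actor with health that can be hitched to the flying pawn and kills it on contact.
; Gravity field scales from the star mesh, and construction applies the star material.
; Obstacles reaching the destruction field subtract their instability from health; at zero the star explodes and tells the game mode it is dead.
; Overlapping the pawn's attach point snaps the star onto it and registers it as carried.
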(event OnComponentBeginOverlap(AttachPoint)
  (params (OverlappedComponent :type Primitive%20Component%20Object%20Reference) (OtherActor :type Actor%20Object%20Reference) (OtherComp :type Primitive%20Component%20Object%20Reference) (OtherBodyIndex :type Integer) (bFromSweep :type Boolean) (SweepResult :type Hit%20Result%20Structure%20%28by%20ref%29))
  ;[1 1 1] Attach TO Trailer hitch
  (bind _asflying_pawn (Utilities|Casting|CastToFlyingPawn OtherActor))
  (if (Class|PrimitiveComponent|IsOverlappingComponent (Variables|Default|GetAttachPoint) (Variables|/Game/FlyingBP/Blueprints/FlyingPawn.FlyingPawn_C|GetStarAttachToPoint _asflying_pawn))
    (Transformation|AttachComponentToComponent (Variables|Default|GetDefaultSceneRoot) (Variables|/Game/FlyingBP/Blueprints/FlyingPawn.FlyingPawn_C|GetStarAttachToPoint _asflying_pawn) "None" "SnapToTarget" "KeepWorld" "KeepWorld" false)
    (Variables|/Game/FlyingBP/Blueprints/FlyingPawn.FlyingPawn_C|SetbHasStar? _asflying_pawn true)
    (Variables|/Game/FlyingBP/Blueprints/FlyingPawn.FlyingPawn_C|SetSetAttachedStar _asflying_pawn self)))

(event OnComponentBeginOverlap(StarDestructionField)
  (params (OverlappedComponent :type Primitive%20Component%20Object%20Reference) (OtherActor :type Actor%20Object%20Reference) (OtherComp :type Primitive%20Component%20Object%20Reference) (OtherBodyIndex :type Integer) (bFromSweep :type Boolean) (SweepResult :type Hit%20Result%20Structure%20%28by%20ref%29))
  ;[1 1 1] Apply damage and explode if need be
  (bind _asobstacles (Utilities|Casting|CastToObstacles OtherActor))
  (if (Class|PrimitiveComponent|IsOverlappingComponent (Variables|Default|GetStarDestructionField) (Variables|/Game/Stars/Obstacles.Obstacles_C|GetGravityCollision _asobstacles))
    (bind _amountofinstability (Default|ApplyUnstability _asobstacles))
    (Default|DestroyObstacle _asobstacles)
    (bind _output_get (Variables|Default|SetHealth (- (Variables|Default|GetHealth) _amountofinstability)))
    (if (<= _output_get 0.0)
      (Game|SpawnActorfromClass "/Game/StarterContent/Blueprints/Blueprint_Effect_Explosion.Blueprint_Effect_Explosion_C" (Math|Transform|MakeTransform (Transformation|GetActorLocation) (Transformation|GetActorRotation) (* (Transformation|GetActorScale3D) "10.000000,10.000000,10.000000")) "Undefined" 0 0)
      (bind _asflying_game_mode (Utilities|Casting|CastToFlyingGameMode (Game|GetGameMode)))
      (Variables|/Game/FlyingBP/Blueprints/FlyingGameMode.FlyingGameMode_C|SetbIsStarAlive? _asflying_game_mode false)
      (Actor|DestroyActor))))

(event OnComponentBeginOverlap(StarMesh)
  (params (OverlappedComponent :type Primitive%20Component%20Object%20Reference) (OtherActor :type Actor%20Object%20Reference) (OtherComp :type Primitive%20Component%20Object%20Reference) (OtherBodyIndex :type Integer) (bFromSweep :type Boolean) (SweepResult :type Hit%20Result%20Structure%20%28by%20ref%29))
  ;[1 1 1] Kill player when hits star
  (bind _asflying_pawn (Utilities|Casting|CastToFlyingPawn OtherActor))
  (if (Class|PrimitiveComponent|IsOverlappingComponent (Variables|Default|GetStarDestructionField) (Variables|/Game/FlyingBP/Blueprints/FlyingPawn.FlyingPawn_C|GetCapsule _asflying_pawn))
    (Default|Death _asflying_pawn)
    (Default|PlayFailureSound _asflying_pawn)
    (Actor|DestroyActor _asflying_pawn)))

(event EventBeginPlay
  ;[1 1 1] Set Gravity field to X times the size of the star
  (Utilities|FlowControl|Sequence
    (:then_0
      (Transformation|SetWorldScale3D (Variables|Default|GetGravityField) (* (Transformation|GetWorldScale (Variables|Default|GetStarMesh)) "2.000000,2.000000,2.000000")))))

(fn ConstructionScript
  (Rendering|Material|SetMaterial (Variables|Default|GetStarMesh) 0 (Variables|Default|GetStarMaterial))
  (Rendering|Material|SetMaterial (Variables|Default|GetAttachPoint) 0 (Variables|Default|GetStarMaterial)))